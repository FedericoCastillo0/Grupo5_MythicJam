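; Inspectable pickup actor that the player can examine up close, rotate with the mouse, then take or put back.
; Interact locks movement and look, shows an InspectExsample widget, and a Timeline lerps the item to the character's ObjetExsample transform.
; Tick polls the widget's Interact flag to trigger Take, which restores control and destroys the actor.
; Cancel restores control, closes the widget and reverses the Timeline.
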(event `self.ReceiveTick`
  (params (DeltaSeconds :type "Float (single-precision)"))
  ;[1 1 1] event tick
  (`|ExecutionSequence`
    (:`then_0`
      (if (`/Game/blueprints/Interact/widget/InspectExsample.interact` (`self.widget`))
        (`self.take`)))
    (:`then_1`
      (if (`self.can inspect`) :!label _label
        (`SceneComponent.K2_AddLocalRotation` (`self.xampleItem`) (`KismetMathLibrary.MakeRotator` (* (stale `InputAxisKey|MouseX` AxisValue) 0.4) (* (stale `InputAxisKey|MouseY` AxisValue) 0.4)) false false)))))

(event `self.ReceiveBeginPlay`
  (bind _xampleitem (`self.xampleItem`))
  ;[1 1 1] beginplay
  (`|ExecutionSequence`
    (:`then_0`
      (set `self.originalDirection` (`SceneComponent.K2_GetComponentLocation` _xampleitem))
      (set `self.originalRotation` (`SceneComponent.K2_GetComponentRotation` _xampleitem))
      (`self.EnableInput` (`GameplayStatics.GetPlayerController` 0)))))

(event `InputAxisKey|MouseX`
  (params (AxisValue :type "Float (single-precision)"))
  ;[1 1 1] event tick
  (goto _label))

(event `InputAxisKey|MouseY`
  (params (AxisValue :type "Float (single-precision)"))
  ;[1 1 1] event tick
  (goto _label))

(event `/Game/blueprints/Interact/Interact_Interface.Interact`
  (bind _xampleitem (`self.xampleItem`))
  ;[1 1 1] Interact
  (`/Engine/EditorBlueprintResources/StandardMacros.DoOnce` false :!label _label_2
    (:`Completed`
      (set `PlayerController.bShowMouseCursor` true (`GameplayStatics.GetPlayerController` 0))
      (set `self.can inspect` true)
      (bind _asbp_first_person_character (cast `/Game/FirstPerson/Blueprints/BP_FirstPersonCharacter` (`GameplayStatics.GetPlayerCharacter` 0)))
      (`CharacterMovementComponent.DisableMovement` (`Character.CharacterMovement` (`GameplayStatics.GetPlayerCharacter` 0)))
      (`Controller.SetIgnoreLookInput` (`GameplayStatics.GetPlayerController` 0) true)
      (`|ExecutionSequence`
        (:`then_0`
          (bind _returnvalue (`|CreateWidget` "/Game/blueprints/Interact/widget/InspectExsample.InspectExsample_C"))
          (bind _output_get (set `self.widget` _returnvalue))
          (`UserWidget.AddToViewport` _output_get 0))
        (:`then_1`
          (bind (_direction _a) (`Timeline|Timeline` :!label _label_3)
            (:`Update`
              (`/Engine/EditorBlueprintResources/StandardMacros.IsValid` _xampleitem
                (:`Is Valid`
                  (bind (_returnvalue_location _returnvalue_rotation) (`KismetMathLibrary.BreakTransform` (`SceneComponent.K2_GetComponentToWorld` (`/Game/FirstPerson/Blueprints/BP_FirstPersonCharacter.objetExsample` _asbp_first_person_character))))
                  (`SceneComponent.K2_SetWorldTransform` _xampleitem (`KismetMathLibrary.MakeTransform` (`KismetMathLibrary.VLerp` (`self.originalDirection`) _returnvalue_location _a) (`KismetMathLibrary.RLerp` (`self.originalRotation`) _returnvalue_rotation _a)) false false))))))))))

(event `EnhancedInput|/Game/FirstPerson/Input/Actions/ia_Cancel`
  (params (ActionValue :type Boolean) (ElapsedSeconds :type "Float (double-precision)") (TriggeredSeconds :type "Float (double-precision)") (InputAction :type "InputAction Object Reference" :default "/Game/FirstPerson/Input/Actions/ia_Cancel.ia_Cancel"))
  (bind _returnvalue (`GameplayStatics.GetPlayerController` 0))
  ;[1 1 1] cancel
  (:`Triggered`
    (`|ExecutionSequence`
      (:`then_0`
        (goto _label_2 :!via `Reset`))
      (:`then_1`
        (if (`self.can inspect`)
          (set `self.can inspect` false)
          (`CharacterMovementComponent.SetMovementMode` (`Character.CharacterMovement` (`GameplayStatics.GetPlayerCharacter` 0)) "MOVE_Walking" 0)
          (set `PlayerController.bShowMouseCursor` false _returnvalue)
          (`Controller.ResetIgnoreLookInput` _returnvalue)
          (`WidgetBlueprintLibrary.SetInputMode_GameOnly` _returnvalue)
          (`|ExecutionSequence`
            (:`then_0`
              (goto _label_3 :!via `Reverse`))
            (:`then_1`
              (`/Game/blueprints/Interact/widget/InspectExsample.cancel_wg` (`self.widget`))
              (`KismetSystemLibrary.PrintText` "Hello"))))))))

(event `take`
  (bind _returnvalue (`GameplayStatics.GetPlayerController` 0))
  (bind _xampleitem (`self.xampleItem`))
  ;[1 1 1] pickUp
  (set `self.can inspect` false)
  (`CharacterMovementComponent.SetMovementMode` (`Character.CharacterMovement` (`GameplayStatics.GetPlayerCharacter` 0)) "MOVE_Walking" 0)
  (set `PlayerController.bShowMouseCursor` false _returnvalue)
  (`Controller.ResetIgnoreLookInput` _returnvalue)
  (`WidgetBlueprintLibrary.SetInputMode_GameOnly` _returnvalue)
  (`|ExecutionSequence`
    (:`then_0`
      (`/Engine/EditorBlueprintResources/StandardMacros.IsValid` _xampleitem
        (:`Is Valid`
          (`ActorComponent.K2_DestroyComponent` _xampleitem)
          (`KismetSystemLibrary.Delay` 0.2)
          (`self.K2_DestroyActor`))))
    (:`then_1`
      (`/Game/blueprints/Interact/widget/InspectExsample.cancel_wg` (`self.widget`)))))

(fn `UserConstructionScript`)