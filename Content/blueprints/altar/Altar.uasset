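; Altar is an interactable that triggers the end screen once the player character has Pergaminos (scrolls).
; Interact reads that value from BP_FirstPersonCharacter and passes through a DoOnce gate so the ending fires a single time.
; After a short delay it shows the Final widget and mouse cursor, disables movement and look input, and pauses the game.
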(event `/Game/blueprints/Interact/Interact_Interface.Interact`
  (if (`KismetMathLibrary.Conv_IntToBool` (`/Game/FirstPerson/Blueprints/BP_FirstPersonCharacter.pergaminos` (cast `/Game/FirstPerson/Blueprints/BP_FirstPersonCharacter` (`GameplayStatics.GetPlayerCharacter` 0) :!pure true)))
    (`/Engine/EditorBlueprintResources/StandardMacros.DoOnce` false
      (:`Completed`
        (`KismetSystemLibrary.Delay` 0.2)
        (bind _returnvalue (`|CreateWidget` "/Game/Finales/FinalBueno/Final.Final_C"))
        (`UserWidget.AddToViewport` _returnvalue 0)
        (set `PlayerController.bShowMouseCursor` true (`GameplayStatics.GetPlayerController` 0))
        (`CharacterMovementComponent.DisableMovement` (`Character.CharacterMovement` (`GameplayStatics.GetPlayerCharacter` 0)))
        (`Controller.SetIgnoreLookInput` (`GameplayStatics.GetPlayerController` 0) true)
        (`GameplayStatics.SetGamePaused` true)))))

(fn `UserConstructionScript`)