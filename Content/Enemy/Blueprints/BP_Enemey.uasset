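; Enemy that wanders near the player, chases on sight and kills the player with a jumpscare.
; It repeatedly moves to random reachable points around the player's current position, retrying on success or failure.
; When PawnSensing sees a pawn, it moves to the player pawn and triggers a one-shot attack on arrival.
; The attack freezes the player, plays a scream animation, switches the view to itself, shows a death screen, then loads the showcase map.
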(event `self.ReceiveBeginPlay`
  (`self.GoToRandomPoint`))

(event `GoToRandomPoint`
  (`|AIMoveTo` self (`NavigationSystemV1.K2_GetRandomReachablePointInRadius` (`SceneComponent.K2_GetComponentLocation` (`Character.Mesh` (`GameplayStatics.GetPlayerCharacter` 0))) 4500.0 null null) null
    (:`OnSuccess`
      _)
    (:`OnFail`
      _))
  (`self.GoToRandomPoint`))

(event `self.PawnSensing.OnSeePawn`
  (params (Pawn :type "Pawn Object Reference"))
  (`|ExecutionSequence`
    (:`then_0`
      (if (not (`self.bIsAttacking`))
        (`|AIMoveTo` self (0.0 0.0 0.0) (`GameplayStatics.GetPlayerPawn` 0)
          (:`OnSuccess`
            (`self.Attack`)))))))

(event `Attack`
  (`/Engine/EditorBlueprintResources/StandardMacros.DoOnce` false
    (:`Completed`
      (`self.DisableInput` (`GameplayStatics.GetPlayerController` 0))
      (`CharacterMovementComponent.DisableMovement` (`Character.CharacterMovement` (cast `/Game/FirstPerson/Blueprints/BP_FirstPersonCharacter` (`GameplayStatics.GetPlayerCharacter` 0) :!pure true)))
      (`SkeletalMeshComponent.PlayAnimation` (`self.Mesh`) "/Game/Enemy/animation/ScreamerBug.ScreamerBug" false)
      (`PlayerController.SetViewTargetWithBlend` (`GameplayStatics.GetPlayerController` 0) (`ActorComponent.GetOwner` (`self.Camera`)) 0.0 "VTBlend_Linear" 0.0 false)
      (`KismetSystemLibrary.Delay` 2.0)
      (bind _returnvalue (`|CreateWidget` "/Game/Enemy/screamer/DeadSenne.DeadSenne_C"))
      (`UserWidget.AddToViewport` _returnvalue 0)
      (`KismetSystemLibrary.Delay` 20.0)
      (`GameplayStatics.OpenLevelBySoftObjectPtr` "/Game/Asian_town/Maps/L_Showcase_map.L_Showcase_map"))))

(fn `UserConstructionScript`)